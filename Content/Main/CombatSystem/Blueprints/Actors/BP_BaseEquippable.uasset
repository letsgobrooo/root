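; Base actor for equippable items in the combat system, such as a sword, that attach to a character.
; GetItemMesh picks the static mesh component if it has a mesh assigned, otherwise the skeletal one.
; OnEquipped sets the equipped flag and snaps the item to the default socket on the owning Character's mesh.
; UnOnEquipped only clears the flag, without detaching the item.
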(fn `AttachActor`
  (params (SocketName :type Name))
  ;[1 1 1] Меш оружия прикрепить к компоненту в указанный сокет
  (`self.K2_AttachToComponent` self (`Character.Mesh` (cast `Character` (`self.GetOwner`) :!pure true)) SocketName "SnapToTarget" "SnapToTarget" "SnapToTarget" true))

(fn `GetIsEquipped`
  (returns (`bIsEquipped?` :type Boolean))
  (return (`self.bIsEquipped?`)))

(fn `GetItemMesh`
  (returns (ReturnValue :type "PrimitiveComponent Object Reference"))
  (bind _itemstaticmesh (`self.ItemStaticMesh`))
  (`/Engine/EditorBlueprintResources/StandardMacros.IsValid` (`StaticMeshComponent.StaticMesh` _itemstaticmesh)
    (:`Is Valid`
      (return _itemstaticmesh))
    (:`Is Not Valid`
      (return (`self.ItemSkeletalMesh`)))))

(fn `OnEquipped`
  ;[1 1 1] Одеть экипировку на персонажа в сокет указанный в имени сокета базового класса Attach Socket Name Default
  (set `self.bIsEquipped?` true)
  (`self.AttachActor` (`self.Attach Socket Name Default`)))

(fn `SetIsEquipped`
  (params (`bIsEquipped?` :type Boolean))
  (set `self.bIsEquipped?` `bIsEquipped?`))

(fn `UnOnEquipped`
  ;[1 1 1] Снять экипировку, если одета
  (if (`self.bIsEquipped?`)
    (set `self.bIsEquipped?` false)))

(fn `UserConstructionScript`)